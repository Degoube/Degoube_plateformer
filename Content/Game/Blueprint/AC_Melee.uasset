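; Actor component that gives the platformer player a melee attack.
; Attack plays the attack montage on the player's mesh, and its notify triggers the hit check while briefly activating the slash Niagara effect.
; The hit check sphere-traces just ahead of the player on Visibility, damages the first actor hit and adds the enemy score value to the GameInstance score, without checking that the target is an enemy.
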(event Custom|Attack
  (bind _bp_player (Variables|Default|GetBp%20player))
  (bind _ns_slash (Variables|/Game/Game/Blueprint/BP_PlayerPlateformer.BP_PlayerPlateformer_C|GetNS_Slash _bp_player))
  (Animation|Montage|PlayMontage (Variables|/Script/Engine.Character|GetMesh (Variables|Default|GetBp%20player)) "/Game/Game/Animation/PlayerAnimation/SwordAnimation/AM_AttackMelee.AM_AttackMelee"
    (:OnNotifyBegin
      (CallFunction|TriggerHit)
      (Components|Activation|SetActive _ns_slash true true)
      (Utilities|FlowControl|Delay 0.2)
      (Components|Activation|SetActive _ns_slash false false))))

(event EventBeginPlay
  (bind _asbp_player_plateformer (Utilities|Casting|CastToBP_PlayerPlateformer (Game|Player|GetPlayerPawn 0)))
  (Variables|Default|SetBp%20player _asbp_player_plateformer))

(fn TriggerHit
  (bind _bp_player (Variables|Default|GetBp%20player))
  (bind _returnvalue (Transformation|GetActorLocation _bp_player))
  (bind (_outhit _returnvalue_2) (Collision|SphereTraceByChannel _returnvalue (+ _returnvalue (* (Transformation|GetActorForwardVector _bp_player) 1.2e+02)) 75.0 "TraceTypeQuery1" false 0 "None"))
  (if _returnvalue_2
    (Game|Damage|ApplyDamage (.HitActor (Collision|BreakHitResult _outhit)) 1.0 0 0)
    (bind _asbp_game_instance (Utilities|Casting|CastToBP_GameInstance (Game|GetGameInstance)))
    (Variables|/Game/Game/Blueprint/BP_GameInstance.BP_GameInstance_C|SetScore _asbp_game_instance (+ (Variables|Default|GetEnnemyScoreValue) (Variables|/Game/Game/Blueprint/BP_GameInstance.BP_GameInstance_C|GetScore _asbp_game_instance)))))