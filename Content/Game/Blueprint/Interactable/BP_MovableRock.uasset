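; BP_MovableRock is an interactable rock that slides away from its starting spot when the player interacts with it.
; On BeginPlay it caches the Scene's world location.
; Interact plays the MovingRock timeline, which lerps an equal negative offset on Y and Z, applied from that cached position through SetActorRelativeTransform.
; Overlapping the Box component tells BP_PlayerPlateformer to show the interact button HUD.
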(event OnComponentBeginOverlap(Box)
  (params (OverlappedComponent :type Primitive%20Component%20Object%20Reference) (OtherActor :type Actor%20Object%20Reference) (OtherComp :type Primitive%20Component%20Object%20Reference) (OtherBodyIndex :type Integer) (bFromSweep :type Boolean) (SweepResult :type Hit%20Result%20Structure%20%28by%20ref%29))
  ;[1 1 1] Show Interact HUD
  (bind _asbp_player_plateformer (Utilities|Casting|CastToBP_PlayerPlateformer OtherActor))
  (Default|InteractButtonHUD _asbp_player_plateformer))

(event EventBeginPlay
  (Variables|Default|SetInitialPosition (Transformation|GetWorldLocation (Variables|Default|GetScene))))

(event Collision|EventActorBeginOverlap
  (params (OtherActor :type Actor%20Object%20Reference)))

(event EventTick
  (params (DeltaSeconds :type Float%20%28single-precision%29)))

(event EventInteract
  (bind _initialposition (Variables|Default|GetInitialPosition))
  ;[1 1 1] Rock interaction
  (bind _rockmoving (Timeline|MovingRock Play)
    (:Update
      (Transformation|SetActorRelativeTransform (Math|Transform|MakeTransform (Math|Vector|MakeVector (.x _initialposition) (+ (.y _initialposition) (Math|Float|Lerp 0.0 -1.5e+02 _rockmoving)) (+ (.z _initialposition) (Math|Float|Lerp 0.0 -1.5e+02 _rockmoving))) "0, 0, 0" "1.000000,1.000000,1.000000") false false))))

(fn ConstructionScript)