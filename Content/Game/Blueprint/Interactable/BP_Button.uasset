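; BP_Button is an interactable button for a light puzzle.
; On Interact it toggles every light in its LightArray, then runs LightChecker to set AllLightOn, stopping at the first unlit light.
; When all of those lights are on, it calls WinLightE on BP_GameInstance to signal the win.
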(event EventBeginPlay)

(event Collision|EventActorBeginOverlap
  (params (OtherActor :type Actor%20Object%20Reference)))

(event EventTick
  (params (DeltaSeconds :type Float%20%28single-precision%29)))

(event EventInteract
  (Utilities|FlowControl|Sequence
    (:then_0
      (for _array_element (Variables|Default|GetLightArray)
        (Default|Toggle _array_element)))
    (:then_1
      (CallFunction|LightChecker)
      (if (Variables|Default|GetAllLightOn)
        (bind _asbp_game_instance (Utilities|Casting|CastToBP_GameInstance (Game|GetGameInstance)))
        (Default|WinLightE _asbp_game_instance)))))

(fn ConstructionScript)

(fn LightChecker
  (bind _array_element (Utilities|Array|ForEachLoopwithBreak (Variables|Default|GetLightArray) :!label _label)
    (:LoopBody
      (if (Variables|/Game/Game/Blueprint/Interactable/BP_Light.BP_Light_C|GetIsOn? _array_element)
        (Variables|Default|SetAllLightOn true)
        (else
          (Variables|Default|SetAllLightOn false)
          (goto _label Break))))))