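; BP_Light is a switchable light in the Interactable folder that holds an on/off state and drives a PointLight component.
; On BeginPlay it sets the starting state from a hard-coded LightID check, so only lights with ID 3 begin lit.
; Its Toggle function flips IsOn and switches the light intensity between MaxIntensity and zero, with no caller inside the Blueprint itself.
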(event EventBeginPlay
  (Utilities|FlowControl|Sequence
    (:then_0
      (if (== (Variables|Default|GetLightID) 3)
        (Variables|Default|SetIsOn? true)
        (Rendering|Components|Light|SetIntensity (Variables|Default|GetPointLight) (Variables|Default|GetMaxIntensity))
        (else
          (Variables|Default|SetIsOn? false)
          (Rendering|Components|Light|SetIntensity (Variables|Default|GetPointLight) 0.0))))))

(fn ConstructionScript)

(fn Toggle
  (bind _pointlight (Variables|Default|GetPointLight))
  (Variables|Default|SetIsOn? (not (Variables|Default|GetIsOn?)))
  (if (Variables|Default|GetIsOn?)
    (Rendering|Components|Light|SetIntensity _pointlight (Variables|Default|GetMaxIntensity))
    (else
      (Rendering|Components|Light|SetIntensity _pointlight 0.0)))
  (return))